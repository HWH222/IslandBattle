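; IB_CameraPawn is a player pawn for mouse-driven ship commands in an AI test setup, showing the cursor on begin play.
; Left click traces under the cursor on the Visibility channel and stores any hit ib_testShip as the selected ship.
; Right click passes the traced location to that ship's CommandMoveTo and spawns a short-lived decal marker there, destroying the previous one.
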(event EventBeginPlay
  (Variables|/Script/Engine.PlayerController|SetbShowMouseCursor (Game|GetPlayerController 0) true))

(event Input|MouseEvents|LeftMouseButton
  (params (Key :type Key%20Structure))
  (bind _returnvalue (Game|GetPlayerController 0))
  (bind (_hitresult _returnvalue_2) (Game|Player|GetHitResultUnderCursorbyChannel _returnvalue "TraceTypeQuery1" false))
  (:Pressed
    (if _returnvalue_2
      (bind _asib_test_ship (Utilities|Casting|CastToib_testShip (.HitActor (Collision|BreakHitResult _hitresult))))
      (Variables|Default|SetSelectedShip _asib_test_ship)
      (Development|PrintString "selected"))))

(event Input|MouseEvents|RightMouseButton
  (params (Key :type Key%20Structure))
  (bind _returnvalue (Game|GetPlayerController 0))
  (bind (_hitresult _returnvalue_2) (Game|Player|GetHitResultUnderCursorbyChannel _returnvalue "TraceTypeQuery1" false))
  (bind _location (Collision|BreakHitResult _hitresult))
  (:Pressed
    (if _returnvalue_2
      (Utilities|IsValid (Variables|Default|GetSelectedShip)
        (:Is%20Valid
          (Utilities|FlowControl|Sequence
            (:then_0
              (Utilities|IsValid (Variables|Default|GetDecalPrevious)
                (:Is%20Valid
                  (Components|DestroyComponent (Variables|Default|GetDecalPrevious)))
                (:Is%20Not%20Valid
                  _))
              (bind _returnvalue_3 (Rendering|Decal|SpawnDecalatLocation "/Game/ArtAssets/M_BaseColor.M_BaseColor" "64.000000,10.000000,10.000000" _location "-90.000000,0.000000,0.000000" 2.0))
              (Variables|Default|SetDecalPrevious _returnvalue_3))
            (:then_1
              (Class|IBShipBase|CommandMoveto (Variables|Default|GetSelectedShip) _location))))))))

(fn ConstructionScript)